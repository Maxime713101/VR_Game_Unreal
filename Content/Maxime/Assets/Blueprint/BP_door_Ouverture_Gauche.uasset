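; Left-opening VR door that swings on its yaw axis while the player holds its GrabComponent with a motion controller.
; Grabbing stores the controller and starts a looping timer on Update_Rotation, which dropping clears.
; Each tick adds the X offset between grab point and controller, computed in the GrabComponent's space, to the Scene's relative yaw, clamped between Minimum and Maximum.
; OuverturePousser (push to open) inverts the rotation direction.
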(event OnGrabbed(GrabComponent)
  (params (Motion%20Controller :type Motion%20Controller%20Component%20Object%20Reference))
  (Variables|Default|SetMotion%20Controller Motion%20Controller)
  (bind _returnvalue (Utilities|Time|SetTimerbyFunctionName 0 "Update_Rotation" 0.01 true))
  (Variables|Default|SetTimer _returnvalue))

(event OnDropped(GrabComponent)
  (Utilities|Time|ClearandInvalidateTimerbyHandle (Variables|Default|GetTimer))
  (Variables|Default|SetMotion%20Controller 0))

(fn ConstructionScript)

(fn UpdateRotation
  (bind _grabcomponent (Variables|Default|GetGrabComponent))
  (bind _motion_controller (Variables|Default|GetMotion%20Controller))
  (bind _scene (Variables|Default|GetScene))
  (bind _scene_2 (Variables|Default|GetScene))
  (bind _returnvalue (Transformation|GetWorldTransform _motion_controller))
  (bind _returnvalue_2 (Transformation|GetWorldTransform _grabcomponent))
  (bind _relativelocation (Variables|/Script/Engine.SceneComponent|GetRelativeLocation _grabcomponent))
  (bind _relativerotation (Variables|/Script/Engine.SceneComponent|GetRelativeRotation _scene))
  (bind _relativerotation_2 (Variables|/Script/Engine.SceneComponent|GetRelativeRotation _scene_2))
  (bind _returnvalue_3 (Math|Transform|MakeRelativeTransform _returnvalue _returnvalue_2))
  (if (Variables|Default|GetOuverture_Pousser)
    (Transformation|SetRelativeRotation _scene (Math|Rotator|MakeRotator (.roll _relativerotation) (.pitch _relativerotation) (Math|Float|Clamp(Float) (+ (.yaw _relativerotation) (* (.x (- _relativelocation (.location _returnvalue_3))) -1.0)) (Variables|Default|GetMinimum) (Variables|Default|GetMaximum))) false false)
    (else
      (Transformation|SetRelativeRotation _scene_2 (Math|Rotator|MakeRotator (.roll _relativerotation_2) (.pitch _relativerotation_2) (Math|Float|Clamp(Float) (+ (.yaw _relativerotation_2) (.x (- _relativelocation (.location _returnvalue_3)))) (Variables|Default|GetMinimum) (Variables|Default|GetMaximum))) false false))))