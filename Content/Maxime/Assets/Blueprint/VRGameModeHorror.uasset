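; VR horror game mode that picks the player's spawn point based on the current level progression.
; ChoosePlayerStart reads LevelValue from GameInstance_Level and maps it to a spawn tag name for the kitchen, child, adult or horror stage.
; It then returns the PlayerStart whose tag matches, printing debug strings along the way.
; BeginPlay, Tick and the construction script are empty.
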(event EventBeginPlay)

(event EventTick
  (params (DeltaSeconds :type Float%20%28single-precision%29)))

(fn ConstructionScript)

(fn ChoosePlayerStart
  (params (Player :type Controller%20Object%20Reference))
  (bind _asgame_instance_level (Utilities|Casting|CastToGameInstance_Level (Game|GetGameInstance)))
  (switch int (Variables|/Game/Levels/GameInstance_Level.GameInstance_Level_C|GetLevelValue _asgame_instance_level)
    (:0
      (bind _output_get (Variables|Default|SetExpectedName "None"))
      (Development|PrintString (Utilities|String|ToString(Name) _output_get)))
    (:1
      (bind _output_get_2 (Variables|Default|SetExpectedName "SpawnCuisine1"))
      (Development|PrintString (Utilities|String|ToString(Name) _output_get_2)))
    (:2
      (bind _output_get_3 (Variables|Default|SetExpectedName "SpawnEnfant2"))
      (Development|PrintString (Utilities|String|ToString(Name) _output_get_3)))
    (:3
      (bind _output_get_4 (Variables|Default|SetExpectedName "SpawnAdulte3"))
      (Development|PrintString (Utilities|String|ToString(Name) _output_get_4)))
    (:4
      (bind _output_get_5 (Variables|Default|SetExpectedName "SpawnHorror4"))
      (Development|PrintString (Utilities|String|ToString(Name) _output_get_5))))
  (bind _outactors (Actor|GetAllActorsOfClass "/Script/Engine.PlayerStart"))
  (for _array_element _outactors
    (if (== (Variables|/Script/Engine.PlayerStart|GetPlayerStartTag _array_element) (Variables|Default|GetExpectedName))
      (return _array_element)
      (else
        (Development|PrintString "Jesuisfaux")))))